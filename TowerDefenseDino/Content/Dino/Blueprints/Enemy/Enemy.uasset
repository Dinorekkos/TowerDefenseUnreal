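; Enemy actor that moves along an array of path points, MyPath, in what appears to be an unfinished state.
; Each Tick, MoveEnemy offsets the location by the current segment's normalized direction times Speed, without delta-time scaling, then tests proximity to the next point.
; That proximity branch is empty, and the CheckLastIndex and DestroyActor calls are unconnected, so the enemy never advances segments or destroys itself.
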(event `self.ReceiveBeginPlay`)

(event `self.ReceiveTick`
  (params (DeltaSeconds :type "Float (single-precision)"))
  (`self.MoveEnemy`)
  (if (< (`KismetMathLibrary.Vector_Distance` (`self.K2_GetActorLocation`) (`|GetArrayItem` (`self.MyPath`) (+ (`self.indexPos`) 1))) 5.0)
    _))

(fn `CheckLastIndex`
  (set `self.indexPos` (+ (`self.indexPos`) 1))
  (if (>= (`self.indexPos`) (`KismetArrayLibrary.Array_LastIndex` (`self.MyPath`)))
    _))

(fn `MoveEnemy`
  (bind _output_get (set `self.direction` (* (`KismetMathLibrary.Normal` (- (`|GetArrayItem` (`self.MyPath`) (+ 1 (`self.indexPos`))) (`|GetArrayItem` (`self.MyPath`) (`self.indexPos`)))) (`self.Speed`))))
  (`self.K2_SetActorLocation` (+ _output_get (`self.K2_GetActorLocation`))))

(fn `UserConstructionScript`)