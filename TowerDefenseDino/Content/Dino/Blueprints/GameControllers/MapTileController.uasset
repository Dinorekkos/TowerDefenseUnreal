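; MapTileController builds the tile map and spawns a single enemy with a route across it on BeginPlay.
; CreateGrid converts flat TileArray indices to grid positions, spawning grass for zeros and another actor for other values, which also become Waypoints map keys for those positions.
; SpawnEnemy looks up waypoints in numeric key order from 2 to the map's length, spawns the enemy at waypoint 2 and assigns the ordered positions as its path.
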(event `self.ReceiveBeginPlay`
  (`self.CreateGrid`)
  (`self.SpawnEnemy`))

(fn `CreateGrid`
  (locals (TileArray :type "Array of Integer"))
  (bind _tilearray (`local.TileArray`))
  (set `self.Grid` _tilearray)
  (for (_array_element _array_index) _tilearray
    (if (== _array_element 0)
      (bind _returnvalue (mod _array_index (`self.GridSize`)))
      (bind _returnvalue_2 (`KismetMathLibrary.Conv_IntToDouble` (* _returnvalue 100)))
      (bind _returnvalue_3 (`KismetMathLibrary.Conv_IntToDouble` (* (/ (- _array_index _returnvalue) (`self.GridSize`)) 100)))
      (bind _returnvalue_4 (`KismetMathLibrary.MakeTransform` (`KismetMathLibrary.MakeVector` _returnvalue_2 _returnvalue_3)))
      (`|SpawnActorFromClass` "/Game/Dino/Blueprints/Floor/GrassTile.GrassTile_C" _returnvalue_4 "Undefined" "MultiplyWithRoot" null null)
      (else
        (`BlueprintMapLibrary.Map_Add` (`self.Waypoints`) (`|GetArrayItem` (`self.Grid`) _array_index) (`KismetMathLibrary.MakeVector` _returnvalue_2 _returnvalue_3))
        (`|SpawnActorFromClass` "/Game/Dino/Blueprints/Floor/RoadTile.RoadTile_C" _returnvalue_4 "Undefined" "MultiplyWithRoot" null null)))))

(fn `SpawnEnemy`
  (bind _waypoints (`self.Waypoints`))
  (bind _value (`BlueprintMapLibrary.Map_Find` (`self.Waypoints`) 2))
  (`BlueprintMapLibrary.Map_Values` _waypoints)
  (for _index (range 2 (+ (`BlueprintMapLibrary.Map_Length` _waypoints) 1))
    (`KismetArrayLibrary.Array_Add` (`self.PathEnemy`) (`BlueprintMapLibrary.Map_Find` (`self.Waypoints`) _index)))
  (bind _returnvalue (`|SpawnActorFromClass` "/Game/Dino/Blueprints/Enemy/Enemy.Enemy_C" (`KismetMathLibrary.MakeTransform` (`KismetMathLibrary.MakeVector` (.x _value) (.y _value) 50.0) (struct :`Yaw` -90.0)) "Undefined" "MultiplyWithRoot" null null))
  (set `/Game/Dino/Blueprints/Enemy/Enemy.MyPath` (`self.PathEnemy`) _returnvalue))

(fn `UserConstructionScript`)